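; Base weapon actor that players pick up through their WeaponSystemComponent, with an overlap-driven interact widget and collision set per weapon state.
; StartFire passes a gate to line-trace from the follow camera, play montage, sound, muzzle, tracer and recoil effects, spend ammo and send damage through CanDamageInterface.
; Manual and automatic reloads block firing for a delay, then refill the magazine from the component's per-ammo-type reserve.
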(event OnComponentBeginOverlap(InteractArea)
  (params (OverlappedComponent :type Primitive%20Component%20Object%20Reference) (OtherActor :type Actor%20Object%20Reference) (OtherComp :type Primitive%20Component%20Object%20Reference) (OtherBodyIndex :type Integer) (bFromSweep :type Boolean) (SweepResult :type Hit%20Result%20Structure%20%28by%20ref%29))
  (bind _weaponstruct (Variables|Default|GetWeaponStruct))
  (bind _widget (Variables|Default|GetWidget))
  (bind (_weaponname _weapontype _weaponenum _weaponclass _magsize _currentammo _damage _weaponimage) (Utilities|Struct|BreakWeaponStruct _weaponstruct))
  ;[1 1 1] Check Weather Weapon Overlap or Not
  (Utilities|Casting|CastToThirdPersonCharacter OtherActor)
  (Variables|Default|SetCanPick? true)
  (Variables|Default|GetInteractWidget
    (:then
      _)
    (:else
      ;;[1 1 1] Create widget UI if You Can Pick
      (bind _returnvalue (UserInterface|CreateWidget "/Game/Game/Blueprints/Weapons/UI/InteractWidget.InteractWidget_C" 0 _weaponname _weapontype _weaponimage))
      (UserInterface|SetWidget _widget _returnvalue)))
  (Rendering|SetVisibility _widget true false))

(event OnComponentEndOverlap(InteractArea)
  (params (OverlappedComponent :type Primitive%20Component%20Object%20Reference) (OtherActor :type Actor%20Object%20Reference) (OtherComp :type Primitive%20Component%20Object%20Reference) (OtherBodyIndex :type Integer))
  ;[1 1 1] Check Weather Weapon Overlap or Not
  (Rendering|SetVisibility (Variables|Default|GetWidget) false false))

(event Custom|StartFire
  (bind (_startpoint _endpoint) (CallFunction|StartandEndPoint))
  (CallFunction|AutoReload)
  (Utilities|FlowControl|Sequence
    (:then_0
      (goto _label Open))
    (:then_1
      (Utilities|FlowControl|Gate true :!label _label
        (:Exit
          (if (> (.CurrentAmmo (Utilities|Struct|BreakWeaponStruct (Variables|Default|GetWeaponStruct))) 0)
            (bind (_outhit _returnvalue) (Collision|LineTraceByChannel _startpoint _endpoint "TraceTypeQuery3" false (Utilities|Array|MakeArray (Variables|Default|GetInteractor)) "None"))
            (CallFunction|WeaponEffects _returnvalue (.ImpactPoint (Collision|BreakHitResult _outhit)) (select _returnvalue (.ImpactPoint (Collision|BreakHitResult _outhit)) (.TraceEnd (Collision|BreakHitResult _outhit))))
            (CallFunction|AmmoCounter)
            (CallFunction|AddDamagetoHitObject (.HitActor (Collision|BreakHitResult _outhit)) _outhit)))))))

(event Custom|stopFire
  (bind (_startpoint _endpoint) (CallFunction|StartandEndPoint))
  (CallFunction|AutoReload)
  (Utilities|FlowControl|Gate true) ; enters at Close
)

(event Custom|ReloadEvent
  (bind _playerref (Variables|Default|GetPlayerRef))
  (Audio|PlaySound2D (Variables|Default|GetReload%20Sound) 1.0 1.0 0.0 0 0)
  (Animation|PlayAnimMontage (Variables|Default|GetPlayerRef) (Variables|Default|GetReload%20Animation) 1.0 "None")
  (Variables|/Game/ThirdPersonBP/Blueprints/ThirdPersonCharacter.ThirdPersonCharacter_C|SetCan%20Fire? _playerref false)
  (Utilities|FlowControl|Delay (Variables|Default|GetReload%20Duration))
  (CallFunction|SetBulletandReload)
  (Variables|/Game/ThirdPersonBP/Blueprints/ThirdPersonCharacter.ThirdPersonCharacter_C|SetCan%20Fire? _playerref true)
  (Variables|Default|SetIsReloading? false))

(event Custom|ReloadButtonEvent
  (bind _weaponstruct (Variables|Default|GetWeaponStruct))
  (bind (_magsize _currentammo) (Utilities|Struct|BreakWeaponStruct _weaponstruct))
  (if (!= (Utilities|Struct|BreakWeaponStruct (Variables|Default|GetWeaponStruct)) 0)
    (if (!= _magsize _currentammo)
      (if (not (Variables|Default|GetIsReloading?))
        (Variables|Default|SetIsReloading? true)
        (CallFunction|ReloadEvent)))))

(event Custom|AutoReload
  (bind _weaponstruct (Variables|Default|GetWeaponStruct))
  (bind (_currentammo _ammotype) (Utilities|Struct|BreakWeaponStruct _weaponstruct))
  (if (and (== _currentammo 0) (> (.Value (Utilities|Map|Find (Variables|/Game/Game/Blueprints/Weapons/WeaponSystemComponent.WeaponSystemComponent_C|GetAmmoType/TotalAmmo (Variables|/Game/ThirdPersonBP/Blueprints/ThirdPersonCharacter.ThirdPersonCharacter_C|GetWeaponSystemComponent (Variables|Default|GetPlayerRef))) _ammotype)) 0))
    (if (not (Variables|Default|GetIsReloading?))
      (Variables|Default|SetIsReloading? true)
      (CallFunction|ReloadEvent))))

(event EventWeaponInteract
  (params (Interactor :type Actor%20Object%20Reference))
  (bind _output_get (Variables|Default|SetInteractor Interactor))
  ;[1 1 1] Interact With Weapon
  (Default|PickupWeapon (Actor|GetComponentbyClass Interactor "/Game/Game/Blueprints/Weapons/WeaponSystemComponent.WeaponSystemComponent_C") self)
  (bind _asthird_person_character (Utilities|Casting|CastToThirdPersonCharacter _output_get))
  (Variables|Default|SetPlayerRef _asthird_person_character))

(fn ConstructionScript
  (bind _weaponstruct (Variables|Default|GetWeaponStruct))
  ;[1 1 1] Set MasterWeapon Constructor
  (Utilities|Struct|SetmembersinWeaponStruct (Variables|Default|GetWeaponStruct) (.weaponname _weaponstruct) (.weapontype _weaponstruct) (.weaponenum _weaponstruct) (Utilities|GetClass self) (.magsize _weaponstruct) (.currentammo _weaponstruct) (.damage _weaponstruct) (.weaponimage _weaponstruct) (.ammotype _weaponstruct)))

(fn SetWeaponState
  (params (WeaponState :type WeaponStateEnum%20Enum :default "NewEnumerator0"))
  (bind _weaponmesh (Variables|Default|GetWeaponMesh))
  (bind _weaponmesh_2 (Variables|Default|GetWeaponMesh))
  (bind _weaponmesh_3 (Variables|Default|GetWeaponMesh))
  (switch Utilities|FlowControl|Switch|SwitchonWeaponStateEnum WeaponState
    (:NewEnumerator0
      (Collision|SetCollisionProfileName (Variables|Default|GetInteractArea) "OverlapAllDynamic" true :!class /Script/Engine.PrimitiveComponent)
      (Collision|SetCollisionProfileName _weaponmesh_2 "DroppedWeapon" true :!class /Script/Engine.PrimitiveComponent)
      (Physics|SetSimulatePhysics _weaponmesh_2 false))
    (:NewEnumerator1
      (Collision|SetCollisionProfileName (Variables|Default|GetInteractArea) "NoCollision" true :!class /Script/Engine.PrimitiveComponent)
      (Collision|SetCollisionProfileName _weaponmesh_3 "NoCollision" true :!class /Script/Engine.PrimitiveComponent)
      (Physics|SetSimulatePhysics _weaponmesh_3 false)
      (Transformation|ResetRelativeTransform _weaponmesh_3))
    (:NewEnumerator2
      (Collision|SetCollisionProfileName (Variables|Default|GetInteractArea) "NoCollision" true :!class /Script/Engine.PrimitiveComponent)
      (Collision|SetCollisionProfileName _weaponmesh "NoCollision" true :!class /Script/Engine.PrimitiveComponent)
      (Physics|SetSimulatePhysics _weaponmesh false))))

(fn StartandEndPoint
  (bind _playerref (Variables|Default|GetPlayerRef))
  (bind _followcamera (Variables|/Game/ThirdPersonBP/Blueprints/ThirdPersonCharacter.ThirdPersonCharacter_C|GetFollowCamera _playerref))
  (return (+ (Transformation|GetWorldLocation _followcamera) (Math|Vector|GetForwardVector (Transformation|GetWorldRotation _followcamera))) (+ (Transformation|GetWorldLocation _followcamera) (* (Math|Vector|GetForwardVector (Transformation|GetWorldRotation _followcamera)) (Variables|Default|GetRange)))))

(fn WeaponEffects
  (params (DoesHit :type Boolean) (ImpactPoint :type Vector) (TraceEnd :type Vector))
  (bind _playerref (Variables|Default|GetPlayerRef))
  (bind _playerref_2 (Variables|Default|GetPlayerRef))
  (bind _weaponsystemcomponent (Variables|/Game/ThirdPersonBP/Blueprints/ThirdPersonCharacter.ThirdPersonCharacter_C|GetWeaponSystemComponent _playerref_2))
  (bind _inhandweapon (Variables|/Game/Game/Blueprints/Weapons/WeaponSystemComponent.WeaponSystemComponent_C|GetInHandWeapon _weaponsystemcomponent))
  (bind _weaponmesh (Variables|MasterWeapon_C|GetWeaponMesh _inhandweapon))
  (bind _returnvalue (Transformation|GetSocketLocation _weaponmesh "Muzzle"))
  (Audio|PlaySound2D (Variables|Default|GetWeapon%20Sound) 1.0 1.0 0.0 0 0)
  (if (Variables|/Game/ThirdPersonBP/Blueprints/ThirdPersonCharacter.ThirdPersonCharacter_C|GetIsAiming? (Variables|Default|GetPlayerRef))
    (Animation|PlayAnimMontage _playerref (Variables|Default|GetAim%20Fire%20Montage) 1.0 "None")
    (else
      (Animation|PlayAnimMontage _playerref (Variables|Default|GetHip%20Fire%20Montage) 1.0 "None")))
  (Effects|SpawnEmitterAttached 0 _weaponmesh "Muzzle" "0, 0, 0" "0, 0, 0" "1.000000,1.000000,1.000000" "SnapToTargetIncludingScale")
  ;[1 1 1] todo
  (Game|SpawnActorfromClass "/Game/Game/Effects/Blueprints/ProjectileTrace.ProjectileTrace_C" (Math|Transform|MakeTransform _returnvalue (Math|Rotator|FindLookatRotation _returnvalue TraceEnd)) "Undefined" 0 0)
  ;[1 1 1] Recoil
  (Pawn|Input|AddControllerPitchInput (Variables|Default|GetPlayerRef) (* (Variables|Default|GetRecoil) -1.0))
  (return))

(fn AmmoCounter
  (bind _weaponstruct (Variables|Default|GetWeaponStruct))
  ;[0.6625 0.3887 1 0.283] Ammo Counter
  (Utilities|Struct|SetmembersinWeaponStruct _weaponstruct (- (.CurrentAmmo (Utilities|Struct|BreakWeaponStruct _weaponstruct)) 1))
  (return))

(fn AddDamagetoHitObject
  (params (HitObject :type Actor%20Object%20Reference) (HitEvent :type Hit%20Result%20Structure))
  (if (Utilities|DoesObjectImplementInterface HitObject "/Game/Game/Blueprints/CanDamageInterface.CanDamageInterface_C")
    (Class|CanDamageInterface|DoDamage(Message) HitObject (.Damage (Utilities|Struct|BreakWeaponStruct (Variables|Default|GetWeaponStruct))) HitEvent)))

(fn SetBulletandReload
  (bind _playerref (Variables|Default|GetPlayerRef))
  (bind _weaponstruct (Variables|Default|GetWeaponStruct))
  (bind _weaponstruct_2 (Variables|Default|GetWeaponStruct))
  (bind _weaponstruct_3 (Variables|Default|GetWeaponStruct))
  (bind _weaponstruct_4 (Variables|Default|GetWeaponStruct))
  (bind (_magsize _currentammo _ammotype) (Utilities|Struct|BreakWeaponStruct _weaponstruct_3))
  (bind _ammotype_2 (Utilities|Struct|BreakWeaponStruct _weaponstruct_4))
  (bind (_magsize_2 _ammotype_3) (Utilities|Struct|BreakWeaponStruct _weaponstruct))
  (bind (_currentammo_2 _ammotype_4) (Utilities|Struct|BreakWeaponStruct _weaponstruct_2))
  (bind _weaponsystemcomponent (Variables|/Game/ThirdPersonBP/Blueprints/ThirdPersonCharacter.ThirdPersonCharacter_C|GetWeaponSystemComponent _playerref))
  (bind _ammotype_totalammo (Variables|/Game/Game/Blueprints/Weapons/WeaponSystemComponent.WeaponSystemComponent_C|GetAmmoType/TotalAmmo _weaponsystemcomponent))
  (bind _value (Utilities|Map|Find _ammotype_totalammo _ammotype_2))
  ;[1 0.9064 0.5413] Check is there enough ammo to reload in inventory and reload
  (if (> (.Value (Utilities|Map|Find (Variables|/Game/Game/Blueprints/Weapons/WeaponSystemComponent.WeaponSystemComponent_C|GetAmmoType/TotalAmmo (Variables|/Game/ThirdPersonBP/Blueprints/ThirdPersonCharacter.ThirdPersonCharacter_C|GetWeaponSystemComponent (Variables|Default|GetPlayerRef))) _ammotype)) 0)
    ;[1 0.9064 0.5413] Check is there enough bullets per round to reload
    (LocalVariables|SetNeededAmmoToReload (- _magsize _currentammo))
    (if (<= _value (LocalVariables|GetNeededAmmoToReload))
      (Utilities|Struct|SetmembersinWeaponStruct (Variables|Default|GetWeaponStruct) (+ _currentammo_2 (.Value (Utilities|Map|Find (Variables|/Game/Game/Blueprints/Weapons/WeaponSystemComponent.WeaponSystemComponent_C|GetAmmoType/TotalAmmo (Variables|/Game/ThirdPersonBP/Blueprints/ThirdPersonCharacter.ThirdPersonCharacter_C|GetWeaponSystemComponent (Variables|Default|GetPlayerRef))) _ammotype_4))))
      (Utilities|Map|Add (Variables|/Game/Game/Blueprints/Weapons/WeaponSystemComponent.WeaponSystemComponent_C|GetAmmoType/TotalAmmo (Variables|/Game/ThirdPersonBP/Blueprints/ThirdPersonCharacter.ThirdPersonCharacter_C|GetWeaponSystemComponent (Variables|Default|GetPlayerRef))) _ammotype_4 0)
      (else
        (Utilities|Struct|SetmembersinWeaponStruct (Variables|Default|GetWeaponStruct) _magsize_2)
        (Utilities|Map|Add (Variables|/Game/Game/Blueprints/Weapons/WeaponSystemComponent.WeaponSystemComponent_C|GetAmmoType/TotalAmmo (Variables|/Game/ThirdPersonBP/Blueprints/ThirdPersonCharacter.ThirdPersonCharacter_C|GetWeaponSystemComponent (Variables|Default|GetPlayerRef))) _ammotype_3 (- _value (LocalVariables|GetNeededAmmoToReload)))))))