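; Weapon inventory component for the player character that handles picking up, holstering, equipping, swapping and dropping weapons.
; PickupWeapon sorts rifles into primary or secondary slots and handguns into the pistol slot, freeing full slots and retrying recursively, then auto-equips.
; Equip acts on WeaponInput, which WeaponTypeAnim validates, to draw, swap or sheathe by reattaching weapons between mesh sockets.
; Weapon state and per-type equipped flags track changes; melee has no pickup path.
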(event Custom|Equip
  (bind _weaponinput (Variables|Default|GetWeaponInput))
  (bind _weaponinput_2 (Variables|Default|GetWeaponInput))
  (bind _weapon (CallFunction|InputBasedonWeapon _weaponinput))
  (if (Utilities|Enum|NotEqual(Enum) (Variables|Default|GetWeaponInput) "NewEnumerator0")
    (if (CallFunction|HasWeaponEquiped)
      (if (Utilities|Enum|NotEqual(Enum) _weaponinput "NewEnumerator4")
        (CallFunction|SwapWeapon _weapon)
        (else
          (CallFunction|Equip/UnEquip _weapon false)
          (Variables|Default|SetRifleWeaponEquiped? false)
          (Variables|Default|SetPistolWeaponEquiped? false)
          (Variables|Default|SetMeleeWeaponEquiped? false)))
      (elif (Utilities|Enum|NotEqual(Enum) _weaponinput_2 "NewEnumerator4")
        (CallFunction|Equip/UnEquip (CallFunction|InputBasedonWeapon _weaponinput_2) true)))))

(event EventBeginPlay
  (bind _asthird_person_character (Utilities|Casting|CastToThirdPersonCharacter (Game|GetPlayerCharacter 0)))
  (Variables|Default|SetPlayerRef _asthird_person_character))

(fn PickupWeapon
  (params (Weapon :type Master%20Weapon%20Object%20Reference))
  ;[0.4566 0.3698 1 0.25] Picking Up the Weapon by Category
  (bind _output_get (Variables|Default|SetInteractingWeapon Weapon))
  (switch Utilities|FlowControl|Switch|SwitchonWeaponEnum (.WeaponEnum (Utilities|Struct|BreakWeaponStruct (Variables|/Game/Game/Blueprints/Weapons/MasterWeapon.MasterWeapon_C|GetWeaponStruct _output_get)))
    (:NewEnumerator1
      (bind _weapon (Utilities|CheckRifelHolsterAvailability (Variables|Default|GetInteractingWeapon) :!label _label)
        (:Slots%20Full
          (CallFunction|PickupWeapon (Variables|Default|GetInteractingWeapon)))
        (:SecondaryWeaponSlotEmpty
          (bind _output_get_2 (Variables|Default|SetSecondaryWeapon _weapon))
          (CallFunction|AttachWeapontoPlayer _output_get_2 (Variables|Default|GetSockettName)))
        (:PrimaryWeaponSlotEmpty
          (bind _output_get_3 (Variables|Default|SetPrimaryWeapon _weapon))
          (CallFunction|AttachWeapontoPlayer _output_get_3 (Variables|Default|GetSockettName)))))
    (:NewEnumerator3
      (goto _label))
    (:NewEnumerator4
      (goto _label))
    (:NewEnumerator5
      (bind _weapon_2 (Utilities|CheckPistolHolsterAvailability (Variables|Default|GetInteractingWeapon) :!label _label_2)
        (:FullPistolHolster
          (CallFunction|PickupWeapon (Variables|Default|GetInteractingWeapon)))
        (:PistolHolsterEmpty
          (bind _output_get_4 (Variables|Default|SetPistolWeapon _weapon_2))
          (CallFunction|AttachWeapontoPlayer _output_get_4 (Variables|Default|GetSockettName)))))
    (:NewEnumerator6
      (goto _label_2))))

(fn AttachWeapontoPlayer
  (params (Weapon :type Master%20Weapon%20Object%20Reference) (Slot :type Name))
  ;[1 1 1] Attaching Weapon to Correct Slot
  (Transformation|AttachComponentToComponent Weapon (Variables|/Script/Engine.Character|GetMesh (Variables|Default|GetPlayerRef)) Slot "SnapToTarget" "SnapToTarget" "SnapToTarget" true)
  (Default|SetWeaponState Weapon "NewEnumerator1")
  (bind _weaponslot (CallFunction|GetSlotBasedonWeapon Weapon))
  (Variables|Default|SetWeaponInput _weaponslot)
  (CallFunction|Equip))

(fn GetSlotBasedonWeapon
  (params (Weapon :type Master%20Weapon%20Object%20Reference))
  ;[0.538 0.1875 1 0.25] If Primary Weapon
  (if (and (Utilities|IsValid (Variables|Default|GetPrimaryWeapon)) (== (Variables|Default|GetPrimaryWeapon) Weapon))
    (return "NewEnumerator1" "PrimaryWeaponSlot")
    (else
      ;[0.05984 1 0 0.25] If Secondary Weapon
      (if (and (Utilities|IsValid (Variables|Default|GetSecondaryWeapon)) (== (Variables|Default|GetSecondaryWeapon) Weapon))
        (return "NewEnumerator2" "SecondaryWeaponSlot")
        (else
          ;[1 0 0.1677 0.25] If Hand Gun
          (if (and (Utilities|IsValid (Variables|Default|GetPistolWeapon)) (== (Variables|Default|GetPistolWeapon) Weapon))
            (return "NewEnumerator5" "PistolSlot")
            (else
              ;[0 0.08442 1 0.25] If Melee Weapon
              (if (and (Utilities|IsValid (Variables|Default|GetMeleeWeapon)) (== (Variables|Default|GetMeleeWeapon) Weapon))
                (return "NewEnumerator3" "MeleeWeaponSlot")))))))))

(fn DropWeapon
  (params (WeaponToDrop :type Master%20Weapon%20Object%20Reference))
  (bind _weaponslot (CallFunction|GetSlotBasedonWeapon WeaponToDrop))
  (LocalVariables|SetWeaponSlot _weaponslot)
  (Transformation|DetachFromActor WeaponToDrop "KeepWorld" "KeepWorld" "KeepWorld")
  (Default|SetWeaponState WeaponToDrop "NewEnumerator0")
  (Variables|Default|SetInHandWeapon 0)
  (switch Utilities|FlowControl|Switch|SwitchonWeaponInputEnum (LocalVariables|GetWeaponSlot)
    (:NewEnumerator1
      (Variables|Default|SetPrimaryWeapon 0)
      (Variables|Default|SetRifleWeaponEquiped? false))
    (:NewEnumerator2
      (Variables|Default|SetSecondaryWeapon 0)
      (Variables|Default|SetRifleWeaponEquiped? false))
    (:NewEnumerator5
      (Variables|Default|SetPistolWeapon 0)
      (Variables|Default|SetPistolWeaponEquiped? false))
    (:NewEnumerator3
      (Variables|Default|SetMeleeWeapon 0)
      (Variables|Default|SetMeleeWeaponEquiped? false)))
  (return))

(fn HasWeaponEquiped
  (return (Math|Boolean|ORBoolean (Variables|Default|GetRifleWeaponEquiped?) (Variables|Default|GetPistolWeaponEquiped?) (Variables|Default|GetMeleeWeaponEquiped?))))

(fn Equip/UnEquip
  (params (The%20Weapon :type Master%20Weapon%20Object%20Reference) (Want%20to%20Equip :type Boolean))
  (bind _weaponslot (CallFunction|GetSlotBasedonWeapon The%20Weapon))
  (LocalVariables|SetThe%20Weapon%20Slot _weaponslot)
  (Transformation|AttachComponentToComponent The%20Weapon (Variables|/Script/Engine.Character|GetMesh (Variables|Default|GetPlayerRef)) (select Want%20to%20Equip "InHandSocket" (Utilities|Select :Index (LocalVariables|GetThe%20Weapon%20Slot) :NewEnumerator0 "None" :NewEnumerator1 "PrimaryWeaponSlot" :NewEnumerator2 "SecondaryWeaponSlot" :NewEnumerator5 "PistolSlot" :NewEnumerator3 "None" :NewEnumerator4 "None")) "SnapToTarget" "SnapToTarget" "SnapToTarget" true)
  (switch Utilities|FlowControl|Switch|SwitchonWeaponInputEnum (LocalVariables|GetThe%20Weapon%20Slot)
    (:NewEnumerator1
      (Variables|Default|SetRifleWeaponEquiped? true))
    (:NewEnumerator2
      (Variables|Default|SetRifleWeaponEquiped? true))
    (:NewEnumerator5
      (Variables|Default|SetPistolWeaponEquiped? true))
    (:NewEnumerator3
      (Variables|Default|SetMeleeWeaponEquiped? true)))
  (if Want%20to%20Equip
    (Variables|Default|SetInHandWeapon The%20Weapon)
    (Default|SetWeaponState The%20Weapon "NewEnumerator2")
    (return)
    (else
      (Default|SetWeaponState The%20Weapon "NewEnumerator1")
      (Variables|Default|SetInHandWeapon 0)
      (Variables|Default|SetRifleWeaponEquiped? false)
      (Variables|Default|SetPistolWeaponEquiped? false)
      (Variables|Default|SetMeleeWeaponEquiped? false)
      (return))))

(fn InputBasedonWeapon
  (params (Weapon%20Input :type WeaponInputEnum%20Enum :default "NewEnumerator0"))
  (bind _primaryweapon (Variables|Default|GetPrimaryWeapon))
  (bind _secondaryweapon (Variables|Default|GetSecondaryWeapon))
  (bind _pistolweapon (Variables|Default|GetPistolWeapon))
  (bind _meleeweapon (Variables|Default|GetMeleeWeapon))
  (bind _inhandweapon (Variables|Default|GetInHandWeapon))
  (switch Utilities|FlowControl|Switch|SwitchonWeaponInputEnum Weapon%20Input
    (:NewEnumerator1
      (Utilities|IsValid _primaryweapon
        (:Is%20Valid
          (return _primaryweapon))))
    (:NewEnumerator2
      (Utilities|IsValid _secondaryweapon
        (:Is%20Valid
          (return _secondaryweapon))))
    (:NewEnumerator5
      (Utilities|IsValid _pistolweapon
        (:Is%20Valid
          (return _pistolweapon))))
    (:NewEnumerator3
      (Utilities|IsValid _meleeweapon
        (:Is%20Valid
          (return _meleeweapon))))
    (:NewEnumerator4
      (Utilities|IsValid _inhandweapon
        (:Is%20Valid
          (return _inhandweapon))))))

(fn WeaponTypeAnim
  (params (WeaponInput :type WeaponInputEnum%20Enum :default "NewEnumerator0"))
  (bind _inhandweapon (Variables|Default|GetInHandWeapon))
  (switch Utilities|FlowControl|Switch|SwitchonWeaponInputEnum WeaponInput
    (:NewEnumerator1
      (Utilities|IsValid (Variables|Default|GetPrimaryWeapon)
        (:Is%20Valid
          _)
        (:Is%20Not%20Valid
          (Variables|Default|SetWeaponInput "NewEnumerator0" :!label _label)
          (return false))))
    (:NewEnumerator2
      (Utilities|IsValid (Variables|Default|GetSecondaryWeapon)
        (:Is%20Valid
          _)
        (:Is%20Not%20Valid
          (goto _label))))
    (:NewEnumerator5
      (Utilities|IsValid (Variables|Default|GetPistolWeapon)
        (:Is%20Valid
          _)
        (:Is%20Not%20Valid
          (goto _label))))
    (:NewEnumerator3
      (Utilities|IsValid (Variables|Default|GetMeleeWeapon)
        (:Is%20Valid
          _)
        (:Is%20Not%20Valid
          (goto _label))))
    (:NewEnumerator4
      (Utilities|IsValid (Variables|Default|GetInHandWeapon)
        (:Is%20Valid
          (Variables|Default|SetWeaponInput "NewEnumerator4")
          (return true)))))
  (Utilities|IsValid _inhandweapon
    (:Is%20Valid
      (bind _weaponslot (CallFunction|GetSlotBasedonWeapon _inhandweapon))
      (if (Utilities|Enum|Equal(Enum) _weaponslot WeaponInput)
        (Variables|Default|SetWeaponInput "NewEnumerator0")
        (return false)
        (else
          _)))
    (:Is%20Not%20Valid
      _))
  (Variables|Default|SetWeaponInput WeaponInput)
  (return true))

(fn SwapWeapon
  (params (TheWeapon :type Master%20Weapon%20Object%20Reference))
  (bind (_weaponslot _slot) (CallFunction|GetSlotBasedonWeapon TheWeapon))
  (LocalVariables|SetNextWeaponSlot _weaponslot)
  (LocalVariables|SetNeaxtWeaponHolster _slot)
  (bind (_weaponslot_2 _slot_2) (CallFunction|GetSlotBasedonWeapon (Variables|Default|GetInHandWeapon)))
  (LocalVariables|SetInHandSlot _weaponslot_2)
  (bind _output_get (LocalVariables|SetInHandHolster _slot_2))
  (Transformation|AttachComponentToComponent (Variables|Default|GetInHandWeapon) (Variables|/Script/Engine.Character|GetMesh (Variables|Default|GetPlayerRef)) _output_get "SnapToTarget" "SnapToTarget" "SnapToTarget" true)
  (Default|SetWeaponState (Variables|Default|GetInHandWeapon) "NewEnumerator1")
  (Variables|Default|SetInHandWeapon 0)
  (Variables|Default|SetRifleWeaponEquiped? false)
  (Variables|Default|SetPistolWeaponEquiped? false)
  (Variables|Default|SetMeleeWeaponEquiped? false)
  (CallFunction|Equip/UnEquip TheWeapon true))