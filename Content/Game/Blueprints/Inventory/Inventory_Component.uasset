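; Inventory component that stores items in a slot array, sized at BeginPlay, and opens the inventory screen.
; AddToInventory tops up a matching partial stack for stackable items, recursing with any overflow; otherwise CreateStack writes into the first empty slot found.
; It always returns true, with no full-inventory check.
; ToggleInventory only opens: it creates a new widget bound to the component, switches to UI-only input and shows the cursor.
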(event EventBeginPlay
  (CallFunction|PrepareInventory))

(event EventTick
  (params (DeltaSeconds :type Float%20%28single-precision%29)))

(fn AddtoInventory
  (params (Content%20To%20Add :type Slot%20Struct%20Structure))
  ;[1 1 1] Add items and item count to inventory
  (if (.isstackable? (.itemstructure Content%20To%20Add))
    ;;[1 1 1] Adding Stackable items
    (bind _stackindex (Utilities|HasPartialStack Content%20To%20Add)
      (:True
        (CallFunction|AddtoStack Content%20To%20Add _stackindex))
      (:False
        ;;[1 1 1] Adding non-stackable items
        (CallFunction|CreateStack Content%20To%20Add :!label _label)))
    (else
      (goto _label)))
  (return true))

(fn PrepareInventory
  ;[1 1 1] resize the inventory if given values are changed
  (Utilities|Array|Resize (Variables|Default|GetInventory) (Variables|Default|GetNumberOfSlots)))

(fn CreateStack
  (params (Content%20To%20Add :type Slot%20Struct%20Structure))
  (bind _inventory (Variables|Default|GetInventory))
  (Utilities|Array|SetArrayElem _inventory (Utilities|Array|FindItem _inventory (Utilities|Struct|MakeSlotStruct "(Name_2_AB56CB1A4194742BFC0A869535FCD3FA=\"\",PickUpSound_5_A692B80F4CAA65FF8A4FD287C485AE50=None,IsStackable?_16_ADBC50004CD0D2EFAC53A79CF26DFF96=False,Thumbnail_10_3DEDF53647A7953373FE029A8127F217=None,Description_13_F30804844CBA9DBED12E61A9E18CD5A7=\"\",InConsumable?_18_8D282EDB4D2BBC632BF293BA93E83501=False,MaxStackSize_22_1C7B75B543CBC81BE6BC54ADB8CC59CE=0,Durability_25_5B0F60C74A8A4AC71C9E9CA187BB0796=0.000000,Item_28_9A2E3C8F441128B9E3F08AA0C409FFC0=None)")) Content%20To%20Add))

(fn AddtoStack
  (params (SlotStruct :type Slot%20Struct%20Structure) (SlotIndex :type Integer))
  (bind _inventory (Variables|Default|GetInventory))
  (bind _inventory_2 (Variables|Default|GetInventory))
  (bind _maxstacksize (Utilities|Struct|BreakItemStruct (.itemstructure SlotStruct)))
  (bind _output (Utilities|Array|Get(acopy) _inventory SlotIndex))
  (bind _output_2 (Utilities|Array|Get(acopy) _inventory_2 SlotIndex))
  (bind _output_get (LocalVariables|SetCurrentQuantity (.quantity _output)))
  (if (> (+ _output_get (.Quantity (Utilities|Struct|BreakSlotStruct SlotStruct))) (.maxstacksize (.itemstructure _output)))
    (Utilities|Array|SetArrayElem (Variables|Default|GetInventory) SlotIndex (Utilities|Struct|MakeSlotStruct (.itemstructure SlotStruct) _maxstacksize))
    (CallFunction|AddtoInventory (Utilities|Struct|MakeSlotStruct (.itemstructure SlotStruct) (- (.quantity SlotStruct) (- _maxstacksize (LocalVariables|GetCurrentQuantity)))))
    (else
      (Utilities|Array|SetArrayElem _inventory_2 SlotIndex (Utilities|Struct|MakeSlotStruct (.itemstructure _output_2) (+ (.quantity _output_2) (.quantity SlotStruct))))))
  (return))

(fn ToggleInventory
  (bind _returnvalue (Game|GetPlayerController 0))
  ;[1 1 1] Toggle inventory
  (bind _returnvalue_2 (UserInterface|CreateWidget "/Game/Game/Blueprints/Inventory/InventoryUI/InventoryWindow.InventoryWindow_C" 0 self))
  (bind _output_get (Variables|Default|SetInventoryWindow _returnvalue_2))
  (UserInterface|Viewport|AddtoViewport _output_get 0)
  (Input|SetInputModeUIOnly _returnvalue 0 "DoNotLock")
  (Variables|/Script/Engine.PlayerController|SetbShowMouseCursor _returnvalue true))