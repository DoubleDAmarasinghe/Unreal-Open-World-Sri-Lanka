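; SoundManager is a trigger-box actor that plays a sequence of dialogue sounds when overlapped, applying a subtitle setting and optionally freezing player movement.
; The box disables its collision, then each 2D sound's finished event advances through the dialogue array.
; Enter stops the current line if skippable.
; After the last line, movement is restored and the actor either re-arms after a delay if repeatable or destroys itself.
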(event OnComponentBeginOverlap(Box)
  (params (OverlappedComponent :type Primitive%20Component%20Object%20Reference) (OtherActor :type Actor%20Object%20Reference) (OtherComp :type Primitive%20Component%20Object%20Reference) (OtherBodyIndex :type Integer) (bFromSweep :type Boolean) (SweepResult :type Hit%20Result%20Structure%20%28by%20ref%29))
  ;[0.2035 0.5312 1 0.454] Dialogue System
  (Class|GameplayStatics|SetSubtitlesEnabled (Variables|Default|GetShowSubtitle?))
  (if (Variables|Default|GetCanMoveWhenPlayDialogue?)
    (Variables|/Game/ThirdPersonBP/Blueprints/ThirdPersonCharacter.ThirdPersonCharacter_C|SetCan%20Move? (Variables|Default|GetPlayer%20ref) true)
    (else
      (Variables|/Game/ThirdPersonBP/Blueprints/ThirdPersonCharacter.ThirdPersonCharacter_C|SetCan%20Move? (Variables|Default|GetPlayer%20ref) false)))
  (Collision|SetCollisionEnabled (Variables|Default|GetBox) "NoCollision")
  (Utilities|Casting|CastToThirdPersonCharacter OtherActor)
  (Input|EnableInput (Game|GetPlayerController 0))
  (bind _returnvalue (Audio|CreateSound2D (Utilities|Array|Get(acopy) (Variables|Default|GetDialougeArray) (Variables|Default|GetCurrentIndex)) 1.0 1.0 0.0 0))
  (Audio|Components|Audio|Play _returnvalue 0.0)
  (EventDispatchers|BindEventtoOnAudioFinished _returnvalue (delegate Custom|CustomEvent_0)))

(event Custom|CustomEvent_0
  ;[0.2035 0.5312 1 0.454] Dialogue System
  (if (== (Utilities|Array|LastIndex (Variables|Default|GetDialougeArray)) (Variables|Default|GetCurrentIndex))
    ;;[0.251 0.238 0.09825 0.708] Check wheather repeatable or not
    (Variables|/Game/ThirdPersonBP/Blueprints/ThirdPersonCharacter.ThirdPersonCharacter_C|SetCan%20Move? (Variables|Default|GetPlayer%20ref) true)
    (if (Variables|Default|GetRepeatable?)
      (Utilities|FlowControl|Delay (Variables|Default|GetDialogue%20Regen%20Time))
      (Collision|SetCollisionEnabled (Variables|Default|GetBox) "QueryOnly")
      (Variables|Default|SetCurrentIndex 0)
      (else
        (Actor|DestroyActor self)))
    (else
      (bind _output_get (Variables|Default|SetCurrentIndex (Variables|Default|GetCurrentIndex)))
      (Math|Integer|IncrementInt _output_get
        (:%20%20
          (bind _returnvalue (Audio|CreateSound2D (Utilities|Array|Get(acopy) (Variables|Default|GetDialougeArray) (Variables|Default|GetCurrentIndex)) 1.0 1.0 0.0 0))
          (Audio|Components|Audio|Play _returnvalue 0.0)
          (EventDispatchers|BindEventtoOnAudioFinished _returnvalue (delegate Custom|CustomEvent_0)))))))

(event EventBeginPlay
  (bind _returnvalue (Actor|GetActorOfClass "/Game/ThirdPersonBP/Blueprints/ThirdPersonCharacter.ThirdPersonCharacter_C"))
  (Variables|Default|SetPlayer%20ref _returnvalue))

(event Input|KeyboardEvents|Enter
  (params (Key :type Key%20Structure :default "None"))
  ;[0.2035 0.5312 1 0.454] Dialogue System
  ;;[0.5342 0.7456 1 0.675] If can skip
  (:Pressed
    (if (Variables|Default|GetSkippable?)
      (Audio|Components|Audio|Stop (stale OnComponentBeginOverlap(Box) _returnvalue)))))

(fn ConstructionScript)