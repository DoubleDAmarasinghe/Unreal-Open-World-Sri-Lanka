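; Pilotable MI17 helicopter pawn that takes possession from the player and hands it back on H.
; A start axis spools RPM, which drives engine sound pitch and the animation blueprint, and enables flight at full RPM.
; Flight axes apply lerp-smoothed movement input for lift, forward and strafe, plus yaw rotation.
; The lift axis event also tilts the root with movement and loops randomized MoveComponentTo drifts to make the body float.
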(event EventBeginPlay
  (bind _ashlicopter_anim_bp (Utilities|Casting|CastToHlicopterAnimBP (Components|SkeletalMesh|GetAnimInstance (Variables|Default|GetMI17))))
  (Variables|Default|SetHelicopterAnim _ashlicopter_anim_bp))

(event Input|AxisEvents|InputAxisHelicopterStart
  (params (AxisValue :type Float%20%28single-precision%29))
  (bind _helicopteranim (Variables|Default|GetHelicopterAnim))
  (bind _helicopter_cue (Variables|Default|GetHelicopter_Cue))
  ;[1 1 1] Helicopter start stop
  (bind _output_get (Variables|Default|Setrpm (Math|Float|Clamp(Float) (+ (Variables|Default|Getrpm) (* AxisValue 0.1)) 0.0 1e+01)))
  (Audio|Parameter|SetFloatParameter _helicopter_cue "Pitch" _output_get :!class /Script/Engine.AudioComponent)
  (Components|Activation|Activate _helicopter_cue false)
  (Utilities|IsValid _helicopteranim
    (:Is%20Valid
      (bind _output_get_2 (Variables|/Game/VigilanteContent/Vehicles/East_Heli_Mi8T/HlicopterAnimBP.HlicopterAnimBP_C|SetRPM _helicopteranim _output_get))
      (if (>= _output_get_2 1e+01)
        (Variables|Default|SetReadyToFly true)
        (else
          (Variables|Default|SetReadyToFly false))))))

(event Input|AxisEvents|InputAxisDroneUp
  (params (AxisValue :type Float%20%28single-precision%29))
  ;[1 1 1] Turn Helicopter
  (if (Variables|Default|GetReadyToFly)
    (bind _output_get (Variables|Default|SetTurn (Math|Float|Lerp AxisValue (Variables|Default|GetTurn) 0.01)))
    (Transformation|SetActorRotation (Math|Rotator|MakeRotator 0.0 0.0 (+ (* _output_get 0.1) (.yaw (Transformation|GetActorRotation)))))))

(event Input|AxisEvents|InputAxisHelicopterUP
  (params (AxisValue :type Float%20%28single-precision%29))
  (bind _returnvalue (Math|Random|RandomFloatinRange -2.0 2.0))
  ;[1 1 1] Move Up Helecopter
  (if (Variables|Default|GetReadyToFly)
    (bind _output_get (Variables|Default|SetHelicopterUp (Math|Float|Lerp (Variables|Default|GetHelicopterUp) (Input|AxisValues|GetHelicopterUP) 0.01)))
    (Pawn|Input|AddMovementInput "0, 0,1.000000" _output_get false)
    (Transformation|SetRelativeRotation (Variables|Default|GetHeliRoot) (Math|Rotator|MakeRotator (* (Variables|Default|Getright) 8.0) (* (Variables|Default|Getfoward) -8.0) 0.0) false false)
    ;[1 1 1] Random float on air
    (Utilities|FlowControl|DoOnce false :!label _label
      (:Completed
        (Components|MoveComponentTo (Variables|Default|GetMI17) (Math|Random|RandomPointinBoundingBox "0, 0,-47.366028" "10.000000,10.000000,10.000000") (Math|Rotator|MakeRotator _returnvalue _returnvalue _returnvalue) true true (Math|Random|RandomFloatinRange 2.0 5.0) false)
        (goto _label Reset)))))

(event Input|AxisEvents|InputAxisMoveForward
  (params (AxisValue :type Float%20%28single-precision%29))
  ;[1 1 1] MOve Forward Helicopter
  (if (Variables|Default|GetReadyToFly)
    (bind _output_get (Variables|Default|Setfoward (Math|Float|Lerp (Variables|Default|Getfoward) AxisValue 0.01)))
    (Pawn|Input|AddMovementInput (Transformation|GetActorForwardVector) _output_get false)))

(event Input|AxisEvents|InputAxisMoveRight
  (params (AxisValue :type Float%20%28single-precision%29))
  ;[1 1 1] Move Right Helicopter
  (if (Variables|Default|GetReadyToFly)
    (bind _output_get (Variables|Default|Setright (Math|Float|Lerp (Variables|Default|Getright) AxisValue 0.01)))
    (Pawn|Input|AddMovementInput (Transformation|GetActorRightVector) _output_get false)))

(event Input|AxisEvents|InputAxisLookUp
  (params (AxisValue :type Float%20%28single-precision%29))
  ;[1 1 1] Mouse Look
  (Pawn|Input|AddControllerPitchInput AxisValue))

(event Input|AxisEvents|InputAxisTurn
  (params (AxisValue :type Float%20%28single-precision%29))
  ;[1 1 1] Mouse Look
  (Pawn|Input|AddControllerYawInput AxisValue))

(event Input|KeyboardEvents|H
  (params (Key :type Key%20Structure :default "None"))
  ;[1 1 1] Toggle Player
  (:Pressed
    (CallFunction|DeactivateHeleicopter)
    (Variables|Default|Setrpm 0.0)))

(fn ConstructionScript)

(fn ActivateHelicopter
  (Pawn|Possess (Game|GetPlayerController 0) self))

(fn DeactivateHeleicopter
  (Pawn|Possess (Game|GetPlayerController 0) (Variables|Default|GetPlayerRef)))